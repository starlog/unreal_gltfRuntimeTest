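; Actor Blueprint that loads a glTF file from disk on BeginPlay and builds its meshes at runtime with glTFRuntime.
; It loops over the asset's nodes, adding a static mesh component for each without applying node transforms.
; Nodes whose names start with "Door" load with default mesh settings.
; All others get complex-as-simple collision and nav collision, so collision behavior follows the node naming convention.
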(event EventBeginPlay
  ;[1 1 1] Start
  (bind _returnvalue (Class|GlTFRuntimeFunctionLibrary|GlTFLoadAssetfromFilename (Variables|Default|GetFileName) false))
  (for _array_element (Class|GlTFRuntimeAsset|GetNodes _returnvalue)
    (if (Utilities|String|StartsWith (.Name (Utilities|Struct|BreakglTFRuntimeNode _array_element)) "Door")
      (CallFunction|GenerateWithoutCollision _returnvalue (.MeshIndex (Utilities|Struct|BreakglTFRuntimeNode _array_element)))
      (else
        (CallFunction|GeneratewithCollision _returnvalue (.MeshIndex (Utilities|Struct|BreakglTFRuntimeNode _array_element)))))))

(fn ConstructionScript)

(fn GenerateWithoutCollision
  (params (glTFObjectRef :type Gl%20TF%20Runtime%20Asset%20Object%20Reference) (meshIndex :type Integer))
  (bind _returnvalue (AddComponent|AddStaticMeshComponent false))
  (bind _returnvalue_2 (Class|GlTFRuntimeAsset|LoadStaticMesh glTFObjectRef meshIndex))
  (Components|StaticMesh|SetStaticMesh _returnvalue _returnvalue_2))

(fn GeneratewithCollision
  (params (glTFObjectRef :type Gl%20TF%20Runtime%20Asset%20Object%20Reference) (meshIndex :type Integer))
  (bind _returnvalue (AddComponent|AddStaticMeshComponent false))
  (bind _returnvalue_2 (Class|GlTFRuntimeAsset|LoadStaticMesh glTFObjectRef meshIndex (Utilities|Struct|MakeglTFRuntimeStaticMeshConfig "ReadWrite" false false true 0 0 "CTF_UseComplexAsSimple" true "Asset" _returnvalue "(CacheMode=ReadWrite,UberMaterialsOverrideMap=(),MaterialsOverrideMap=(),MaterialsOverrideByNameMap=(),TexturesOverrideMap=(),ImagesOverrideMap=(),bDisableVertexColors=False,bGeneratesMipMaps=False,bMergeSectionsByMaterial=False,SpecularFactor=0.000000,bMaterialsOverrideMapInjectParams=False,ParamsMultiplier=(),ImagesConfig=(Compression=TC_Default,Group=TEXTUREGROUP_World,bSRGB=False,MaxWidth=0,MaxHeight=0,bVerticalFlip=False,bForceHDR=False,bCompressMips=False,bStreaming=False,LODBias=0),Variant=\"\",bSkipLoad=False,VertexColorOnlyMaterial=None,ScalarParamsOverrides=(),bLoadMipMaps=False)" 0 "" 0 "IfMissing" "IfMissing" false false false true)))
  (Components|StaticMesh|SetStaticMesh _returnvalue _returnvalue_2))